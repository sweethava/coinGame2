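; Player state that owns the player's health, death and respawn cycle.
; ApplyDamage lowers health with an on-screen readout, camera shake and sound, then CheckHealth triggers KillPlayer at zero.
; KillPlayer notifies the ABP_Movement anim instance, disables movement and starts a timer to RespawnPlayer.
; RespawnPlayer replaces the character at SpawnPoint, possesses it, calls RestartGame on BP_GameState and resets health, always using player index 0.
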(fn ConstructionScript)

(fn ApplyDamage
  (params (damage :type Float%20%28double-precision%29))
  ;[1 1 1] Применение урона
  (if (not (Variables|Default|Getdead))
    (bind _output_get (Variables|Default|Sethealth (- (Variables|Default|Gethealth) damage)))
    (Development|PrintString (Utilities|String|Append (Utilities|String|ToString(Float) _output_get) "HP") true true "(R=1.000000,G=0.097246,B=0.000000,A=1.000000)")
    (Game|Feedback|ClientStartCameraShake (Game|GetPlayerController 0) "/Game/MyGame/Blueprints/BP_DamageCameraShake.BP_DamageCameraShake_C" 3.0 "CameraLocal" "0, 0, 0")
    (Audio|PlaySound2D "/Game/MyGame/Audio/Damage/A_Damage_Cue.A_Damage_Cue" 1.0 1.0 0.0 0 0)
    (CallFunction|CheckHealth)))

(fn CheckHealth
  ;[1 1 1] Проверка уровня здоровья игрока и его убийство
  (if (and (<= (Variables|Default|Gethealth) 0.0) (not (Variables|Default|Getdead)))
    (CallFunction|KillPlayer)))

(fn KillPlayer
  ;[1 1 1] Смерть игрока и вызов респавна
  (Variables|Default|Setdead true)
  (bind _asbp_third_person_character (Utilities|Casting|CastToBP_ThirdPersonCharacter (Game|GetPlayerCharacter 0)))
  (bind _output_get (LocalVariables|Setplayer _asbp_third_person_character))
  (bind _asabp_movement (Utilities|Casting|CastToABP_Movement (Components|SkeletalMesh|GetAnimInstance (Variables|/Script/Engine.Character|GetMesh _output_get))))
  (Default|KillCharacter _asabp_movement)
  (Pawn|Components|CharacterMovement|DisableMovement (Variables|/Script/Engine.Character|GetCharacterMovement (LocalVariables|Getplayer)))
  (Utilities|Time|SetTimerbyFunctionName 0 "respawnPlayer" 5.0))

(fn RespawnPlayer
  ;[1 1 1] Респавн и сброс здоровья
  (bind _asbp_third_person_character (Utilities|Casting|CastToBP_ThirdPersonCharacter (Game|GetPlayerCharacter 0)))
  (Actor|DestroyActor _asbp_third_person_character)
  (bind _returnvalue (Game|SpawnActorfromClass "/Game/ThirdPerson/Blueprints/BP_ThirdPersonCharacter.BP_ThirdPersonCharacter_C" (Math|Transform|MakeTransform (LocalVariables|GetspawnPoint)) "Undefined" 0 0))
  (Pawn|Possess (Game|GetPlayerController 0) _returnvalue)
  (bind _asbp_game_state (Utilities|Casting|CastToBP_GameState (Game|GetGameState)))
  (Default|RestartGame _asbp_game_state)
  (Variables|Default|Setdead false)
  (Variables|Default|Sethealth 1e+02))