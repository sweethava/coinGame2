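; Game state Blueprint that spawns, tracks and reports coin collection.
; On BeginPlay, RestartGame spawns a BP_Coin at each CoinCoords entry, then stores the number of coin actors in the level as a byte total, without resetting the collected count.
; PickUpCoin destroys the coin, increments the count and calls CheckProgress, which prints progress plus an all-collected message shown on screen when the totals match.
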(event EventBeginPlay
  (CallFunction|RestartGame))

(fn ConstructionScript)

(fn CountCoins
  ;[1 1 1] Считаем количество коинов
  (bind _outactors (Actor|GetAllActorsOfClass "/Game/MyGame/Blueprints/BP_Coin.BP_Coin_C"))
  (Variables|Default|SetallCoins (Math|Conversions|ToByte(Integer) (Utilities|Array|Length _outactors))))

(fn PickUpCoin
  (params (coin :type BP%20Coin%20Object%20Reference))
  (Actor|DestroyActor coin)
  (Variables|Default|SetcollectedCoins (+ (Variables|Default|GetcollectedCoins) 1))
  (CallFunction|CheckProgress))

(fn CheckProgress
  (Development|PrintString (Utilities|String|Append (Utilities|String|ToString(Byte) (Variables|Default|GetcollectedCoins)) "/" (Utilities|String|ToString(Byte) (Variables|Default|GetallCoins))) true true "(R=0.000000,G=0.660000,B=1.000000,A=1.000000)" 3.0)
  (Development|PrintString "All coins collected" (== (Variables|Default|GetcollectedCoins) (Variables|Default|GetallCoins)) true "(R=0.000000,G=1.000000,B=0.521752,A=1.000000)" 5.0))

(fn RestartGame
  (for _array_element (Variables|Default|GetcoinCoords)
    (Game|SpawnActorfromClass "/Game/MyGame/Blueprints/BP_Coin.BP_Coin_C" (Math|Conversions|ToTransform(Vector) _array_element) "Undefined" 0 0))
  (CallFunction|CountCoins))